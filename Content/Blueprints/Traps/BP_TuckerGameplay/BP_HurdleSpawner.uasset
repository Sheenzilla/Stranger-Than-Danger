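; BP_HurdleSpawner is a trap actor that spawns BP_Obstacle_Base hurdles at the location of its Sphere component.
; HurdleTrapon and HurdleTrapOff toggle whether SpawnHurdle is allowed to spawn.
; After each spawn, a flag blocks further spawns for a random whole-second delay of a few seconds.
; Nothing in this graph calls SpawnHurdle, so it does not repeat on its own.
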(event `/Game/Blueprints/Traps/BPI_trapControl.hurdleTrapOn`
  (set `self.canSpawnHurdle` true))

(event `/Game/Blueprints/Traps/BPI_trapControl.hurdleTrapOff`
  (set `self.canSpawnHurdle` false))

(event `/Game/Blueprints/Traps/BPI_trapControl.spawnHurdle`
  (if (`self.canSpawnHurdle`)
    (if (not (`self.HurdleIsSpawned`))
      (set `self.HurdleIsSpawned` true)
      (`|SpawnActorFromClass` "/Game/Blueprints/Traps/BP_TuckerGameplay/BP_Obstacle_Base.BP_Obstacle_Base_C" (`KismetMathLibrary.MakeTransform` (`SceneComponent.K2_GetComponentLocation` (`self.Sphere`))) "Undefined" "OverrideRootScale")
      (`KismetSystemLibrary.Delay` (`KismetMathLibrary.Conv_IntToDouble` (`KismetMathLibrary.RandomIntegerInRange` 1 4)))
      (set `self.HurdleIsSpawned` false))))

(fn `UserConstructionScript`)