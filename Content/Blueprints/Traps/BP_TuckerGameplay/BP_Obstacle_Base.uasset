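; BP_Obstacle_Base is a base trap obstacle actor whose displayed mesh comes from a StaticMeshToDisplay variable, applied in the construction script.
; When CubeCollider overlaps anything other than the player character, the actor destroys itself after a fixed delay.
; Player overlaps have no effect here, and Tick applies a zero local offset, so the actor does not move by itself.
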(event `self.ReceiveTick`
  (params (DeltaSeconds :type "Float (single-precision)"))
  (`self.K2_AddActorLocalOffset` (`KismetMathLibrary.MakeVector` 0.0)))

(event `self.CubeCollider.OnComponentBeginOverlap`
  (params (OverlappedComponent :type "PrimitiveComponent Object Reference") (OtherActor :type "Actor Object Reference") (OtherComp :type "PrimitiveComponent Object Reference") (OtherBodyIndex :type Integer) (bFromSweep :type Boolean) (SweepResult :type "HitResult Structure (by ref)"))
  ;[1 1 1] Player Collision
  (if (not (== (`GameplayStatics.GetPlayerCharacter` 0) OtherActor))
    ;[1 1 1] Non-Player Collision
    (`KismetSystemLibrary.Delay` 7.0)
    (`self.K2_DestroyActor`)))

(fn `UserConstructionScript`
  (`StaticMeshComponent.SetStaticMesh` (`self.ObstacleMesh`) (`self.StaticMeshToDisplay`)))