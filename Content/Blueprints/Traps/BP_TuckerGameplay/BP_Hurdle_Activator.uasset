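; A trigger volume actor that switches the hurdle trap on while the player stands inside its MenuCollider and off when they leave.
; On begin and end overlap with player 0's character, it sends HurdleTrapOn or HurdleTrapOff messages to that character.
; It then finds every BP_HurdleSpawner in the level with GetAllActorsOfClass and relays the same message to each.
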(event `self.MenuCollider.OnComponentBeginOverlap`
  (params (OverlappedComponent :type "PrimitiveComponent Object Reference") (OtherActor :type "Actor Object Reference") (OtherComp :type "PrimitiveComponent Object Reference") (OtherBodyIndex :type Integer) (bFromSweep :type Boolean) (SweepResult :type "HitResult Structure (by ref)"))
  ;[1 1 1] Tells the player and any hurdle spawner than the hurdle trap is enabled
  (if (== OtherActor (`GameplayStatics.GetPlayerCharacter` 0))
    (`|ExecutionSequence`
      (:`then_0`
        (message `/Game/Blueprints/Traps/BPI_trapControl.hurdleTrapOn` (`GameplayStatics.GetPlayerCharacter` 0)))
      (:`then_1`
        (bind _outactors (`GameplayStatics.GetAllActorsOfClass` "/Game/Blueprints/Traps/BP_TuckerGameplay/BP_HurdleSpawner.BP_HurdleSpawner_C"))
        (for _array_element _outactors
          (message `/Game/Blueprints/Traps/BPI_trapControl.hurdleTrapOn` _array_element))))))

(event `self.MenuCollider.OnComponentEndOverlap`
  (params (OverlappedComponent :type "PrimitiveComponent Object Reference") (OtherActor :type "Actor Object Reference") (OtherComp :type "PrimitiveComponent Object Reference") (OtherBodyIndex :type Integer))
  ;[1 1 1] Tells the player and any hurdle spawner than the hurdle trap is enabled
  (if (== OtherActor (`GameplayStatics.GetPlayerCharacter` 0))
    (`|ExecutionSequence`
      (:`then_0`
        (message `/Game/Blueprints/Traps/BPI_trapControl.hurdleTrapOff` (`GameplayStatics.GetPlayerCharacter` 0)))
      (:`then_1`
        (bind _outactors (`GameplayStatics.GetAllActorsOfClass` "/Game/Blueprints/Traps/BP_TuckerGameplay/BP_HurdleSpawner.BP_HurdleSpawner_C"))
        (for _array_element _outactors
          (message `/Game/Blueprints/Traps/BPI_trapControl.hurdleTrapOff` _array_element))))))

(fn `UserConstructionScript`)