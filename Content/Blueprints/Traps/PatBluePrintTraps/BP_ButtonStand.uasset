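; Button stand that lets the player open the blender trap doors while standing in range.
; Box overlap tracks the player, toggles the PressButton prompt and sends trap on/off messages to the player character.
; When BlenderInteract fires during overlap, it sends the open-doors message to every actor implementing BPI_trapControl, avoiding direct trap references.
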(event `/Game/Blueprints/Traps/BPI_trapControl.blenderInteract`
  ;[1 1 1] activate trap when the player hits a certain button
  (if (`self.IsOverlapping`)
    (bind _outactors (`GameplayStatics.GetAllActorsWithInterface` "/Game/Blueprints/Traps/BPI_trapControl.BPI_trapControl_C"))
    (for _array_element _outactors
      (message `/Game/Blueprints/Traps/BPI_trapControl.openBlenderDoors` _array_element))))

(event `self.Box.OnComponentBeginOverlap`
  (params (OverlappedComponent :type "PrimitiveComponent Object Reference") (OtherActor :type "Actor Object Reference") (OtherComp :type "PrimitiveComponent Object Reference") (OtherBodyIndex :type Integer) (bFromSweep :type Boolean) (SweepResult :type "HitResult Structure (by ref)"))
  (bind _returnvalue (`GameplayStatics.GetPlayerCharacter` 0))
  ;[1 1 1] If Player is Overlapped, trap can be used
  (if (== OtherActor (`GameplayStatics.GetPlayerCharacter` 0))
    (set `self.IsOverlapping` true)
    (if (`self.IsOverlapping`) :!label _label
      (`|ExecutionSequence`
        (:`then_0`
          (`SceneComponent.SetVisibility` (`self.PressButton`) true false))
        (:`then_1`
          (message `/Game/Blueprints/Traps/BPI_trapControl.blenderTrapOn` _returnvalue)))
      (else
        (`|ExecutionSequence`
          (:`then_0`
            (`SceneComponent.SetVisibility` (`self.PressButton`) false false))
          (:`then_1`
            (message `/Game/Blueprints/Traps/BPI_trapControl.blenderTrapOff` _returnvalue)))))))

(event `self.Box.OnComponentEndOverlap`
  (params (OverlappedComponent :type "PrimitiveComponent Object Reference") (OtherActor :type "Actor Object Reference") (OtherComp :type "PrimitiveComponent Object Reference") (OtherBodyIndex :type Integer))
  ;[1 1 1] If Player is Overlapped, trap can be used
  (if (== OtherActor (`GameplayStatics.GetPlayerCharacter` 0))
    (set `self.IsOverlapping` false)
    (goto _label)))

(fn `UserConstructionScript`)