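; BP_checkerTrapButton is an overlap trigger that switches the checkered floor trap on while the player stands in it and off when they leave.
; Entering reveals a text render and adds a newly created BPW_checkerHUD widget to the viewport; leaving hides the text and removes the widget.
; Both overlap events broadcast the matching on or off message to every actor implementing BPI_trapControl, found through a world-wide interface search.
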(event `self.ReceiveActorBeginOverlap`
  (params (OtherActor :type "Actor Object Reference"))
  (if (== OtherActor (`GameplayStatics.GetPlayerCharacter` 0))
    (`SceneComponent.SetHiddenInGame` (`self.TextRender`) false false)
    (bind _returnvalue (`|CreateWidget` "/Game/Blueprints/Traps/CheckeredFloor_Trap_BPs/BPW_checkerHUD.BPW_checkerHUD_C"))
    (`UserWidget.AddToViewport` _returnvalue 0)
    (bind _outactors (`GameplayStatics.GetAllActorsWithInterface` "/Game/Blueprints/Traps/BPI_trapControl.BPI_trapControl_C"))
    (for _array_element _outactors
      (message `/Game/Blueprints/Traps/BPI_trapControl.checkeredTrapOn` _array_element))))

(event `self.ReceiveActorEndOverlap`
  (params (OtherActor :type "Actor Object Reference"))
  (if (== OtherActor (`GameplayStatics.GetPlayerCharacter` 0))
    (`SceneComponent.SetHiddenInGame` (`self.TextRender`) true false)
    (`Widget.RemoveFromParent` (stale `self.ReceiveActorBeginOverlap` _returnvalue))
    (bind _outactors (`GameplayStatics.GetAllActorsWithInterface` "/Game/Blueprints/Traps/BPI_trapControl.BPI_trapControl_C"))
    (for _array_element _outactors
      (message `/Game/Blueprints/Traps/BPI_trapControl.checkeredTrapOff` _array_element))))

(fn `UserConstructionScript`)