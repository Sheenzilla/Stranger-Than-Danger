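; Checkered trap floor piece that, while enabled, randomly turns red, blue or green every three seconds.
; Events switch the trap on and off and select which single color is lethal.
; Tick applies the material and, when an overlapping player meets the lethal color, broadcasts that color's destroy message to all BPI_trapControl actors.
; Collision volume overlaps track contact with interface-implementing actors and broadcast it likewise.
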(event `/Game/STD_GameContent/BPs_TestingChambers/BP_PatrickFtraps/BPI_trapControl.checkeredTrapOn`
  ;[1 1 1] Proximity to this trap's button will activate these events
  (set `self.trapIsEnabled` true))

(event `/Game/STD_GameContent/BPs_TestingChambers/BP_PatrickFtraps/BPI_trapControl.checkeredTrapOff`
  ;[1 1 1] Proximity to this trap's button will activate these events
  (set `self.trapIsEnabled` false))

(event `self.ReceiveTick`
  (params (DeltaSeconds :type "Float (single-precision)"))
  (bind _damaging_color (`self.Damaging Color`))
  (if (`self.trapIsEnabled`)
    (`|ExecutionSequence`
      (:`then_0`
        ;[1 1 1] Every three seconds set the checker box to Red Green or Blue at RANDOM
        (`KismetSystemLibrary.Delay` 3.0)
        (set `self.BlockColor` (`KismetMathLibrary.RandomIntegerInRange` 0 2)))
      (:`then_1`
        (if (== (`self.BlockColor`) 0)
          (`PrimitiveComponent.SetMaterial` (`self.Checker Box`) 0 "/Game/STD_GameContent/BPs_TestingChambers/CheckeredFloor_Trap_BPs/RedMat.RedMat")
          (set `self.Damaging Color` 0)
          (elif (== (`self.BlockColor`) 1)
            (`PrimitiveComponent.SetMaterial` (`self.Checker Box`) 0 "/Game/STD_GameContent/BPs_TestingChambers/CheckeredFloor_Trap_BPs/BlueMat.BlueMat")
            (set `self.Damaging Color` 1)
            (else
              (`PrimitiveComponent.SetMaterial` (`self.Checker Box`) 0 "/Game/STD_GameContent/BPs_TestingChambers/CheckeredFloor_Trap_BPs/GreenMat.GreenMat")
              (set `self.Damaging Color` 2)))))
      (:`then_2`
        (if (`self.IsOverlappingPlayer?`)
          ;[1 1 1] Kill the player he/she is if both in contact with the checkerbox and the checkerbox is set as lethal to the player
          (if (and (== 0 _damaging_color) (`self.RedIsActive`))
            (bind _outactors (`GameplayStatics.GetAllActorsWithInterface` "/Game/STD_GameContent/BPs_TestingChambers/BP_PatrickFtraps/BPI_trapControl.BPI_trapControl_C"))
            (for _array_element _outactors
              (message `/Game/STD_GameContent/BPs_TestingChambers/BP_PatrickFtraps/BPI_trapControl.destroyForRed` _array_element))
            (elif (and (== 1 _damaging_color) (`self.BlueIsActive`))
              (bind _outactors_2 (`GameplayStatics.GetAllActorsWithInterface` "/Game/STD_GameContent/BPs_TestingChambers/BP_PatrickFtraps/BPI_trapControl.BPI_trapControl_C"))
              (for _array_element_2 _outactors_2
                (message `/Game/STD_GameContent/BPs_TestingChambers/BP_PatrickFtraps/BPI_trapControl.destroyForBlue` _array_element_2))
              (elif (and (== 2 _damaging_color) (`self.GreenIsActive`))
                (bind _outactors_3 (`GameplayStatics.GetAllActorsWithInterface` "/Game/STD_GameContent/BPs_TestingChambers/BP_PatrickFtraps/BPI_trapControl.BPI_trapControl_C"))
                (for _array_element_3 _outactors_3
                  (message `/Game/STD_GameContent/BPs_TestingChambers/CheckeredFloor_Trap_BPs/Player_BPI.DestroyForGreen` _array_element_3))))))))))

(event `/Game/STD_GameContent/BPs_TestingChambers/BP_PatrickFtraps/BPI_trapControl.damageColorRed`
  ;[1 1 1] When 1 2 or 3 is pressed, set corisponding color as leathal
  (if (`self.trapIsEnabled`)
    (`|ExecutionSequence`
      (:`then_0`
        (set `self.RedIsActive` true))
      (:`then_1`
        (set `self.BlueIsActive` false))
      (:`then_2`
        (set `self.GreenIsActive` false)))))

(event `/Game/STD_GameContent/BPs_TestingChambers/BP_PatrickFtraps/BPI_trapControl.damageColorBlue`
  ;[1 1 1] When 1 2 or 3 is pressed, set corisponding color as leathal
  (if (`self.trapIsEnabled`)
    (`|ExecutionSequence`
      (:`then_0`
        (set `self.RedIsActive` false))
      (:`then_1`
        (set `self.BlueIsActive` true))
      (:`then_2`
        (set `self.GreenIsActive` false)))))

(event `/Game/STD_GameContent/BPs_TestingChambers/BP_PatrickFtraps/BPI_trapControl.damageColorGreen`
  ;[1 1 1] When 1 2 or 3 is pressed, set corisponding color as leathal
  (if (`self.trapIsEnabled`)
    (`|ExecutionSequence`
      (:`then_0`
        (set `self.RedIsActive` false))
      (:`then_1`
        (set `self.BlueIsActive` false))
      (:`then_2`
        (set `self.GreenIsActive` true)))))

(event `self.Collision Volume.OnComponentBeginOverlap`
  (params (OverlappedComponent :type "PrimitiveComponent Object Reference") (OtherActor :type "Actor Object Reference") (OtherComp :type "PrimitiveComponent Object Reference") (OtherBodyIndex :type Integer) (bFromSweep :type Boolean) (SweepResult :type "HitResult Structure (by ref)"))
  ;[1 1 1] Overlap event control for when the player touches the checkerbox (this is used to validate when the player can be killed)
  (if (`KismetSystemLibrary.DoesImplementInterface` OtherActor "/Game/STD_GameContent/BPs_TestingChambers/BP_PatrickFtraps/BPI_trapControl.BPI_trapControl_C")
    (`|ExecutionSequence`
      (:`then_0`
        (set `self.IsOverlappingPlayer?` true))
      (:`then_1`
        (bind _outactors (`GameplayStatics.GetAllActorsWithInterface` "/Game/STD_GameContent/BPs_TestingChambers/BP_PatrickFtraps/BPI_trapControl.BPI_trapControl_C"))
        (for _array_element _outactors
          (message `/Game/STD_GameContent/BPs_TestingChambers/BP_PatrickFtraps/BPI_trapControl.isOverlappingChecker` _array_element))))))

(event `self.Collision Volume.OnComponentEndOverlap`
  (params (OverlappedComponent :type "PrimitiveComponent Object Reference") (OtherActor :type "Actor Object Reference") (OtherComp :type "PrimitiveComponent Object Reference") (OtherBodyIndex :type Integer))
  ;[1 1 1] Overlap event control for when the player touches the checkerbox (this is used to validate when the player can be killed)
  (if (`KismetSystemLibrary.DoesImplementInterface` OtherActor "/Game/STD_GameContent/BPs_TestingChambers/BP_PatrickFtraps/BPI_trapControl.BPI_trapControl_C")
    (`|ExecutionSequence`
      (:`then_0`
        (set `self.IsOverlappingPlayer?` false))
      (:`then_1`
        (bind _outactors (`GameplayStatics.GetAllActorsWithInterface` "/Game/STD_GameContent/BPs_TestingChambers/BP_PatrickFtraps/BPI_trapControl.BPI_trapControl_C"))
        (for _array_element _outactors
          (message `/Game/STD_GameContent/BPs_TestingChambers/BP_PatrickFtraps/BPI_trapControl.notOverlappingChecker` _array_element))))))

(fn `UserConstructionScript`)