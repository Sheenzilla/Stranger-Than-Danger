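; BP_ButtonStand is a button stand that lets the player trigger trap doors while standing within its box.
; Box overlap events set IsOverlapping, toggle the PressButton prompt's visibility and message the player character about entering or leaving.
; When EHasBeenPressed fires during overlap, it broadcasts OpenPlease to every actor implementing BPI_TrapDoorEvent, so the stand holds no direct door references.
; EIsPressed is a stub that always returns false.
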(event `/Game/STD_GameContent/BPs_TestingChambers/PatBluePrintTraps/BPI_PlayerToButton.EHasBeenPressed`
  ;[1 1 1] activate trap when the player hits a certain button
  (if (`self.IsOverlapping`)
    (bind _outactors (`GameplayStatics.GetAllActorsWithInterface` "/Game/STD_GameContent/BPs_TestingChambers/PatBluePrintTraps/BPI_TrapDoorEvent.BPI_TrapDoorEvent_C"))
    (message `/Game/STD_GameContent/BPs_TestingChambers/PatBluePrintTraps/BPI_TrapDoorEvent.OpenPlease` _outactors)))

(event `self.Box.OnComponentBeginOverlap`
  (params (OverlappedComponent :type "PrimitiveComponent Object Reference") (OtherActor :type "Actor Object Reference") (OtherComp :type "PrimitiveComponent Object Reference") (OtherBodyIndex :type Integer) (bFromSweep :type Boolean) (SweepResult :type "HitResult Structure (by ref)"))
  ;[1 1 1] If Player is Overlapped, trap can be used
  (if (== OtherActor (`GameplayStatics.GetPlayerCharacter` 0))
    (set `self.IsOverlapping` true)
    (if (`self.IsOverlapping`) :!label _label
      (`|ExecutionSequence`
        (:`then_0`
          (`SceneComponent.SetVisibility` (`self.PressButton`) true false))
        (:`then_1`
          (message `/Game/STD_GameContent/BPs_TestingChambers/PatBluePrintTraps/BPI_PlayerToButton.PlayerHasOverlapped` (`GameplayStatics.GetPlayerCharacter` 0))))
      (else
        (`|ExecutionSequence`
          (:`then_0`
            (`SceneComponent.SetVisibility` (`self.PressButton`) false false))
          (:`then_1`
            (message `/Game/STD_GameContent/BPs_TestingChambers/PatBluePrintTraps/BPI_PlayerToButton.PlayerIsNotOverlapping` (`GameplayStatics.GetPlayerCharacter` 0))))))))

(event `self.Box.OnComponentEndOverlap`
  (params (OverlappedComponent :type "PrimitiveComponent Object Reference") (OtherActor :type "Actor Object Reference") (OtherComp :type "PrimitiveComponent Object Reference") (OtherBodyIndex :type Integer))
  ;[1 1 1] If Player is Overlapped, trap can be used
  (if (== OtherActor (`GameplayStatics.GetPlayerCharacter` 0))
    (set `self.IsOverlapping` false)
    (goto _label)))

(fn `EIsPressed`
  (returns (Pressed :type Boolean))
  (return false))

(fn `UserConstructionScript`)