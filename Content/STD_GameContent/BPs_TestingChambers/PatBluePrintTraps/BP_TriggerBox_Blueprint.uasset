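; Trigger box that lets the player open trap doors with a press while standing inside it.
; Player begin and end overlap set IsOverlapping and toggle the ButtonText prompt's visibility.
; EHasBeenPressed, if the player is overlapping, gathers every BPI_TrapDoorEvent actor and sends OpenPleaseMessage, so it is not linked to one specific door.
; EIsPressed is a stub that always returns false.
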(event `/Game/STD_GameContent/BPs_TestingChambers/PatBluePrintTraps/BPI_PlayerToButton.EHasBeenPressed`
  (if (`self.IsOverlapping`)
    (bind _outactors (`GameplayStatics.GetAllActorsWithInterface` "/Game/STD_GameContent/BPs_TestingChambers/PatBluePrintTraps/BPI_TrapDoorEvent.BPI_TrapDoorEvent_C"))
    (message `/Game/STD_GameContent/BPs_TestingChambers/PatBluePrintTraps/BPI_TrapDoorEvent.OpenPlease` _outactors)))

(event `self.CollisionComponent.OnComponentBeginOverlap`
  (params (OverlappedComponent :type "PrimitiveComponent Object Reference") (OtherActor :type "Actor Object Reference") (OtherComp :type "PrimitiveComponent Object Reference") (OtherBodyIndex :type Integer) (bFromSweep :type Boolean) (SweepResult :type "HitResult Structure (by ref)"))
  (if (== OtherActor (`GameplayStatics.GetPlayerCharacter` 0))
    (set `self.IsOverlapping` true)
    (if (`self.IsOverlapping`) :!label _label
      (`SceneComponent.ToggleVisibility` (`self.ButtonText`) false)
      (else
        (`SceneComponent.ToggleVisibility` (`self.ButtonText`) false)))))

(event `self.CollisionComponent.OnComponentEndOverlap`
  (params (OverlappedComponent :type "PrimitiveComponent Object Reference") (OtherActor :type "Actor Object Reference") (OtherComp :type "PrimitiveComponent Object Reference") (OtherBodyIndex :type Integer))
  (if (== OtherActor (`GameplayStatics.GetPlayerCharacter` 0))
    (set `self.IsOverlapping` false)
    (goto _label)))

(fn `EIsPressed`
  (returns (Pressed :type Boolean))
  (return false))

(fn `UserConstructionScript`)