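; BP_wallTrap is a wall trap for the testing chambers that plays a level sequence animation when triggered.
; Walltrapon and WalltrapOff, driven by a wall trap button, set a proximity flag that must be true for WallTrapInteract to fire.
; Interacting creates and plays the sequence, with an active flag and a delay blocking retriggering until it finishes.
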(event `/Game/STD_GameContent/BPs_TestingChambers/BP_PatrickFtraps/BPI_trapControl.wallTrapInteract`
  ;[1 1 1] Check for trap activity, if it is not active, set active then play animation
  (if (`self.wallTrapIsNear`)
    (if (not (`self.wallTrapIsActive`))
      (set `self.wallTrapIsActive` true)
      (bind _returnvalue (`LevelSequencePlayer.CreateLevelSequencePlayer` "/Game/TrapSecquence.TrapSecquence"))
      (`LevelSequencePlayer.Play` _returnvalue)
      (`KismetSystemLibrary.Delay` 3.25)
      (set `self.wallTrapIsActive` false))))

(event `/Game/STD_GameContent/BPs_TestingChambers/BP_PatrickFtraps/BPI_trapControl.walltrapOn`
  ;[1 1 1] massage sent from wallTrapButton - player must be near for this trap to activate
  (set `self.wallTrapIsNear` true))

(event `/Game/STD_GameContent/BPs_TestingChambers/BP_PatrickFtraps/BPI_trapControl.walltrapOff`
  ;[1 1 1] massage sent from wallTrapButton - player must be near for this trap to activate
  (set `self.wallTrapIsNear` false))

(fn `UserConstructionScript`)