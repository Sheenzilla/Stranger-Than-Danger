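; Proximity button that arms wall traps in a testing chamber while the player stands near it.
; When the player character enters or leaves its Box trigger, it finds every actor implementing BPI_trapControl and sends WalltrapOnMessage or WalltrapOffMessage.
; The broadcast goes to all implementers in the level rather than a linked trap.
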(event `self.Box.OnComponentBeginOverlap`
  (params (OverlappedComponent :type "PrimitiveComponent Object Reference") (OtherActor :type "Actor Object Reference") (OtherComp :type "PrimitiveComponent Object Reference") (OtherBodyIndex :type Integer) (bFromSweep :type Boolean) (SweepResult :type "HitResult Structure (by ref)"))
  ;[1 1 1] when the player is near this button, the wall trap can be activated
  (if (== OtherActor (`GameplayStatics.GetPlayerCharacter` 0))
    (bind _outactors (`GameplayStatics.GetAllActorsWithInterface` "/Game/STD_GameContent/BPs_TestingChambers/BP_PatrickFtraps/BPI_trapControl.BPI_trapControl_C"))
    (for _array_element _outactors
      (message `/Game/STD_GameContent/BPs_TestingChambers/BP_PatrickFtraps/BPI_trapControl.walltrapOn` _array_element))))

(event `self.Box.OnComponentEndOverlap`
  (params (OverlappedComponent :type "PrimitiveComponent Object Reference") (OtherActor :type "Actor Object Reference") (OtherComp :type "PrimitiveComponent Object Reference") (OtherBodyIndex :type Integer))
  ;[1 1 1] when the player is near this button, the wall trap can be activated
  (if (== OtherActor (`GameplayStatics.GetPlayerCharacter` 0))
    (bind _outactors (`GameplayStatics.GetAllActorsWithInterface` "/Game/STD_GameContent/BPs_TestingChambers/BP_PatrickFtraps/BPI_trapControl.BPI_trapControl_C"))
    (for _array_element _outactors
      (message `/Game/STD_GameContent/BPs_TestingChambers/BP_PatrickFtraps/BPI_trapControl.walltrapOff` _array_element))))

(fn `UserConstructionScript`)