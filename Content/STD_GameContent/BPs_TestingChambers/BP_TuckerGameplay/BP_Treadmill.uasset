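; BP_Treadmill is a testing-chamber treadmill that pushes the player along negative world X while they stand in its collider.
; ColliderBox begin and end overlap events set a flag for player character 0 only.
; While the flag is set, Tick feeds the player's world location, minus a fixed X step, into SetActorRelativeLocation without sweep.
; The step is per frame, unscaled by delta time, and ignores the treadmill's rotation.
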(event `self.ReceiveTick`
  (params (DeltaSeconds :type "Float (single-precision)"))
  (bind _returnvalue (`GameplayStatics.GetPlayerCharacter` 0))
  (bind (_returnvalue_x _returnvalue_y _returnvalue_z) (`KismetMathLibrary.BreakVector` (`self.K2_GetActorLocation` _returnvalue)))
  ;[1 1 1] Treadmill Movement
  (if (`self.IsOverlappingPlayer`)
    (`self.K2_SetActorRelativeLocation` _returnvalue (`KismetMathLibrary.MakeVector` (+ -3.0 _returnvalue_x) _returnvalue_y _returnvalue_z) false false)))

(event `self.ColliderBox.OnComponentBeginOverlap`
  (params (OverlappedComponent :type "PrimitiveComponent Object Reference") (OtherActor :type "Actor Object Reference") (OtherComp :type "PrimitiveComponent Object Reference") (OtherBodyIndex :type Integer) (bFromSweep :type Boolean) (SweepResult :type "HitResult Structure (by ref)"))
  ;[1 1 1] Treadmill Movement
  (if (== OtherActor (`GameplayStatics.GetPlayerCharacter` 0))
    (set `self.IsOverlappingPlayer` true)))

(event `self.ColliderBox.OnComponentEndOverlap`
  (params (OverlappedComponent :type "PrimitiveComponent Object Reference") (OtherActor :type "Actor Object Reference") (OtherComp :type "PrimitiveComponent Object Reference") (OtherBodyIndex :type Integer))
  (if (== OtherActor (`GameplayStatics.GetPlayerCharacter` 0))
    (set `self.IsOverlappingPlayer` false)))

(fn `UserConstructionScript`)