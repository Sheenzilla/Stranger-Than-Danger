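; Trigger volume Blueprint that switches a spike trap on and off as the player enters and leaves it.
; Box overlap begin and end events check whether the other actor is player character 0.
; On a match they send the activated or deactivated spike message to the player character itself through a Blueprint Interface, with no direct reference to a trap actor.
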(event `self.Box.OnComponentBeginOverlap`
  (params (OverlappedComponent :type "PrimitiveComponent Object Reference") (OtherActor :type "Actor Object Reference") (OtherComp :type "PrimitiveComponent Object Reference") (OtherBodyIndex :type Integer) (bFromSweep :type Boolean) (SweepResult :type "HitResult Structure (by ref)"))
  ;[1 1 1] Activates function from BPI
  (if (== OtherActor (`GameplayStatics.GetPlayerCharacter` 0))
    (message `/Game/STD_GameContent/BPs_TestingChambers/BP_meganTrap/BPI_TrapControl3.ActivatedSpike` (`GameplayStatics.GetPlayerCharacter` 0))))

(event `self.Box.OnComponentEndOverlap`
  (params (OverlappedComponent :type "PrimitiveComponent Object Reference") (OtherActor :type "Actor Object Reference") (OtherComp :type "PrimitiveComponent Object Reference") (OtherBodyIndex :type Integer))
  ;[1 1 1] Deactivates function from BPI
  (if (== OtherActor (`GameplayStatics.GetPlayerCharacter` 0))
    (message `/Game/STD_GameContent/BPs_TestingChambers/BP_meganTrap/BPI_TrapControl3.DeactivatedSpike` (`GameplayStatics.GetPlayerCharacter` 0))))

(fn `UserConstructionScript`)