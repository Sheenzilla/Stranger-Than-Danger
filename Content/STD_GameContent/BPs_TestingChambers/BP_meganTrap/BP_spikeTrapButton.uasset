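; Spike trap button in a testing chamber that lets the player spawn short-lived boxes at preset target points while standing near it.
; A Box trigger tracks player overlap and sends the player character on/off messages through a Blueprint Interface.
; The primary and secondary interact events each spawn a BP_Box at the first fake target point actor of their own class, with a five-second lifespan.
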(event `/Game/STD_GameContent/BPs_TestingChambers/BP_PatrickFtraps/BPI_trapControl.spiketrapSecondaryInteract`
  ;[1 1 1] Spawn block 1 if player is near the button
  (if (`self.Overlapping`)
    (bind _outactors (`GameplayStatics.GetAllActorsOfClass` "/Game/STD_GameContent/BPs_TestingChambers/BP_meganTrap/BP_FakeTargetPoint.BP_FakeTargetPoint_C"))
    (set `self.fakeTarget` (`KismetArrayLibrary.Array_Get` _outactors))
    (bind _returnvalue (`|SpawnActorFromClass` "/Game/STD_GameContent/BPs_TestingChambers/BP_meganTrap/BP_Box.BP_Box_C" (`KismetMathLibrary.Conv_VectorToTransform` (`SceneComponent.K2_GetComponentLocation` (`/Game/STD_GameContent/BPs_TestingChambers/BP_meganTrap/BP_FakeTargetPoint.DefaultSceneRoot` (`self.fakeTarget`)))) "Undefined" "OverrideRootScale"))
    (`self.SetLifeSpan` _returnvalue 5.0)))

(event `/Game/STD_GameContent/BPs_TestingChambers/BP_PatrickFtraps/BPI_trapControl.spiketrapInteract`
  ;[1 1 1] Spawn block 2 if player is near the button
  (if (`self.Overlapping`)
    (bind _outactors (`GameplayStatics.GetAllActorsOfClass` "/Game/STD_GameContent/BPs_TestingChambers/BP_meganTrap/BP_FakeTargetPoint2.BP_FakeTargetPoint2_C"))
    (set `self.fakeTarget2` (`KismetArrayLibrary.Array_Get` _outactors))
    (bind _returnvalue (`|SpawnActorFromClass` "/Game/STD_GameContent/BPs_TestingChambers/BP_meganTrap/BP_Box.BP_Box_C" (`KismetMathLibrary.Conv_VectorToTransform` (`SceneComponent.K2_GetComponentLocation` (`/Game/STD_GameContent/BPs_TestingChambers/BP_meganTrap/BP_FakeTargetPoint2.DefaultSceneRoot` (`self.fakeTarget2`)))) "Undefined" "OverrideRootScale"))
    (`self.SetLifeSpan` _returnvalue 5.0)))

(event `self.Box.OnComponentBeginOverlap`
  (params (OverlappedComponent :type "PrimitiveComponent Object Reference") (OtherActor :type "Actor Object Reference") (OtherComp :type "PrimitiveComponent Object Reference") (OtherBodyIndex :type Integer) (bFromSweep :type Boolean) (SweepResult :type "HitResult Structure (by ref)"))
  ;[1 1 1] Activates function from BPI
  (if (== OtherActor (`GameplayStatics.GetPlayerCharacter` 0))
    (set `self.overlapping` true)
    (message `/Game/STD_GameContent/BPs_TestingChambers/BP_PatrickFtraps/BPI_trapControl.spikeTrapOn` (`GameplayStatics.GetPlayerCharacter` 0))))

(event `self.Box.OnComponentEndOverlap`
  (params (OverlappedComponent :type "PrimitiveComponent Object Reference") (OtherActor :type "Actor Object Reference") (OtherComp :type "PrimitiveComponent Object Reference") (OtherBodyIndex :type Integer))
  ;[1 1 1] Deactivates function from BPI
  (if (== OtherActor (`GameplayStatics.GetPlayerCharacter` 0))
    (set `self.overlapping` false)
    (message `/Game/STD_GameContent/BPs_TestingChambers/BP_PatrickFtraps/BPI_trapControl.spiketrapOff` (`GameplayStatics.GetPlayerCharacter` 0))))

(fn `UserConstructionScript`)